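; BP_RKBase is a player character Blueprint that handles Enhanced Input movement, look and jump.
; On BeginPlay it runs the parent logic, fetches and caches the RKMan player controller through a message call, then adds the IMC_RKMan mapping context.
; Move input follows the capsule's forward and right vectors, look input drives controller yaw and pitch, and jump input calls Jump.
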(event `self.ReceiveBeginPlay`
  ;[1 1 1] Add Mapping Context
  (`parent.ReceiveBeginPlay`)
  (bind _pc_rkman (message `/Game/Blueprints/Interface/IF_GetPlayerController.GetPlayerControllerRef` (`GameplayStatics.GetPlayerController` 0)))
  (`/Engine/EditorBlueprintResources/StandardMacros.IsValid` _pc_rkman
    (:`Is Valid`
      (bind _output_get (set `self.PC RKMan` _pc_rkman))
      (`EnhancedInputSubsystemInterface.AddMappingContext` (pcsubsystem `EnhancedInputLocalPlayerSubsystem` _output_get) "/Game/Blueprints/Input/IMC_RKMan.IMC_RKMan" 0 (struct)))))

(event `EnhancedInput|/Game/Blueprints/Input/IA_RKMove`
  (params (ActionValue :type "Vector2D Structure") (ElapsedSeconds :type "Float (double-precision)") (TriggeredSeconds :type "Float (double-precision)") (InputAction :type "InputAction Object Reference" :default "/Game/Blueprints/Input/IA_RKMove.IA_RKMove"))
  ;[1 1 1] Movement
  (:`Triggered`
    (`self.AddMovementInput` (`SceneComponent.GetForwardVector` (`self.CapsuleComponent`)) ActionValue_X)
    (`self.AddMovementInput` (`SceneComponent.GetRightVector` (`self.CapsuleComponent`)) ActionValue_Y)))

(event `EnhancedInput|/Game/Blueprints/Input/IA_RKLook`
  (params (ActionValue :type "Vector2D Structure") (ElapsedSeconds :type "Float (double-precision)") (TriggeredSeconds :type "Float (double-precision)") (InputAction :type "InputAction Object Reference" :default "/Game/Blueprints/Input/IA_RKLook.IA_RKLook"))
  (:`Triggered`
    (`self.AddControllerYawInput` ActionValue_X)
    (`self.AddControllerPitchInput` ActionValue_Y)))

(event `EnhancedInput|/Game/Blueprints/Input/IA_RKJump`
  (params (ActionValue :type Boolean) (ElapsedSeconds :type "Float (double-precision)") (TriggeredSeconds :type "Float (double-precision)") (InputAction :type "InputAction Object Reference" :default "/Game/Blueprints/Input/IA_RKJump.IA_RKJump"))
  (:`Triggered`
    (`self.Jump`)))

(fn `UserConstructionScript`)